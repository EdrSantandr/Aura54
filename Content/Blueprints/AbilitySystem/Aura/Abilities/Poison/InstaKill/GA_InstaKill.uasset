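; GA_InstaKill is a poison-folder gameplay ability that, as wired, only prints a debug message on activation and never ends itself.
; A disconnected chain, apparently reused from Firebolt, gets target data under the mouse, turns the avatar toward it and plays the Firebolt cast montage.
; That chain commits, waits on the Firebolt montage event without handling it, and ends with the montage.
; No kill or damage logic is present.
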(event `self.K2_ActivateAbility`
  (`KismetSystemLibrary.PrintString` "instakill activated"))