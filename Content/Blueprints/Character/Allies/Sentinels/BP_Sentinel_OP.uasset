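; BP_Sentinel_OP is an allied Sentinel variant that uses a RotatingMovement component to rotate around an offset pivot.
; On BeginPlay it runs the parent logic, then passes the vector from itself to player 0's pawn into SetPivotRotation.
; That function writes the vector to the component's PivotTranslation, once, with no later updates.
; Tick and the construction script only call their parents.
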(event `self.ReceiveBeginPlay`
  (`parent.ReceiveBeginPlay`)
  (`self.SetPivotRotation` (- (`self.K2_GetActorLocation` (`Controller.K2_GetPawn` (`GameplayStatics.GetPlayerController` 0))) (`self.K2_GetActorLocation`))))

(event `self.ReceiveTick`
  (params (DeltaSeconds :type "Float (single-precision)"))
  (`parent.ReceiveTick` DeltaSeconds))

(fn `SetPivotRotation`
  (params (InPivotRotation :type "Vector Structure"))
  (set `RotatingMovementComponent.PivotTranslation` InPivotRotation (`self.RotatingMovement`)))

(fn `UserConstructionScript`
  (`parent.UserConstructionScript`))