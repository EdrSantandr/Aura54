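; Passive mana siphon gameplay ability for the Aura ability system, applying a gameplay effect to its owner when activated.
; Activation builds a level 1 spec from the GameplayEffectClass variable through the avatar's ability system component and applies it.
; Activation and end only print debug messages otherwise, with no effect removal in this graph.
; A delayed cooldown-commit and EndAbility chain is disconnected, so the ability never ends itself.
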(event `self.K2_ActivateAbility`
  (`KismetSystemLibrary.PrintString` "manasiphon activated" true true (struct :`R` 1.0 :`G` 0.092126 :`A` 1.0) 4.0)
  (`self.K2_ApplyGameplayEffectSpecToOwner` (`AbilitySystemComponent.MakeOutgoingSpec` :`self` (`AbilitySystemBlueprintLibrary.GetAbilitySystemComponent` (`self.GetAvatarActorFromActorInfo`)) :`GameplayEffectClass` (`self.Gameplay Effect Class`) :`Level` 1.0)))

(event `self.K2_OnEndAbility`
  (params (bWasCancelled :type Boolean))
  (`KismetSystemLibrary.PrintString` "MANAsiphon DEACTRIVATED" true true (struct :`R` 1.0 :`G` 0.9575 :`A` 1.0) 4.0))