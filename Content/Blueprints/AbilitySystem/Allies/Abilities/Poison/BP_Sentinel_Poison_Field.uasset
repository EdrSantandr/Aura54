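; Sentinel ally poison field actor that slows characters inside it for a limited lifetime.
; Overlapping characters are tracked; those implementing CombatInterface get flagged as slowed, with walk speed and ground friction scaled down.
; Leaving the sphere restores flagged characters, and destruction resets every tracked one.
; Original movement values live in one shared pair of variables, overwritten by each new slow, rather than stored per character.
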(event `self.ReceiveBeginPlay`
  (`self.SetInitialLifetime`))

(event `self.ReceiveActorBeginOverlap`
  (params (OtherActor :type "Actor Object Reference"))
  (bind _ascharacter (cast `Character` OtherActor))
  (bind _output_get (set `self.OverlappedCharacter` _ascharacter))
  (`KismetArrayLibrary.Array_AddUnique` (`self.SlowedCharacters`) _output_get)
  (if (`KismetSystemLibrary.DoesImplementInterface` _output_get "/Script/Aura.CombatInterface")
    (`self.SetActorSlow`)))

(event `self.Sphere.OnComponentEndOverlap`
  (params (OverlappedComponent :type "PrimitiveComponent Object Reference") (OtherActor :type "Actor Object Reference") (OtherComp :type "PrimitiveComponent Object Reference") (OtherBodyIndex :type Integer))
  (bind _ascharacter (cast `Character` OtherActor))
  (if (`KismetSystemLibrary.DoesImplementInterface` _ascharacter "/Script/Aura.CombatInterface")
    (`self.ResetActorSlow` _ascharacter)))

(event `self.ReceiveDestroyed`
  (for _array_element (`self.SlowedCharacters`)
    (`self.ResetActorSlow` _array_element)))

(fn `ResetActorSlow`
  (params (InCharacter :type "Character Object Reference"))
  (bind _charactermovement (`Character.CharacterMovement` InCharacter))
  (bind _returnvalue (message `CombatInterface.GetIsSlowed` InCharacter))
  (if _returnvalue
    (set `CharacterMovementComponent.MaxWalkSpeed` (`self.OriginalMaxWalkSpeed`) _charactermovement)
    (set `CharacterMovementComponent.GroundFriction` (`self.OriginalGroundFriction`) _charactermovement)
    (message `CombatInterface.SetIsSlowed` InCharacter false)))

(fn `SetActorSlow`
  (bind _charactermovement (`Character.CharacterMovement` (`self.OverlappedCharacter`)))
  (bind _charactermovement_2 (`Character.CharacterMovement` (`self.OverlappedCharacter`)))
  (message `CombatInterface.SetIsSlowed` (`self.OverlappedCharacter`) true)
  (set `self.OriginalMaxWalkSpeed` (`CharacterMovementComponent.MaxWalkSpeed` _charactermovement_2))
  (set `self.OriginalGroundFriction` (`CharacterMovementComponent.GroundFriction` _charactermovement_2))
  (set `CharacterMovementComponent.MaxWalkSpeed` (* (`self.OriginalMaxWalkSpeed`) (`self.SlowSpeedPercentage`)) _charactermovement)
  (set `CharacterMovementComponent.GroundFriction` (* (`self.OriginalGroundFriction`) (`self.SlowFrictionPercentage`)) _charactermovement))

(fn `SetInitialLifetime`
  (`self.SetLifeSpan` (+ (`KismetMathLibrary.RandomFloatInRange` 0.5 0.5) (`self.Lifetime`)))
  (`KismetArrayLibrary.Array_Clear` (`self.SlowedCharacters`)))

(fn `UserConstructionScript`)