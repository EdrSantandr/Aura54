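; Base enchant gameplay ability that lets the player cast onto a highlighted ally, triggered on input release.
; A cast montage event switches to confirm input mapping and enters a casting loop that zeroes walk speed while awaiting confirm or cancel.
; Confirming on an AllyInterface actor turns the avatar toward it, plays a confirm montage, then calls EnchantAlly and commits on its event.
; Every handled exit restores movement and input mapping before ending.
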(event `self.K2_ActivateAbility`
  (bind _highlightedactor (`self.HighlightedActor`))
  (`AbilityTask_WaitInputRelease.WaitInputRelease` false
    (:`OnRelease`
      (`self.StoreOwnerVariables`)
      (`AbilityTask_PlayMontageAndWait.CreatePlayMontageAndWaitProxy` "None" "/Game/Assets/Characters/Aura/Animations/Abilities/AM_Cast_Enchant.AM_Cast_Enchant"
        (:`then`
          (`AbilityTask_WaitGameplayEvent.WaitGameplayEvent` (struct :`TagName` "Event.Montage.CastEnchant") null
            (:`EventReceived`
              (`self.ChangeToConfirmInputMapping`)
              (`self.InCastingLoop`)
              (`AbilityTask_WaitConfirmCancel.WaitConfirmCancel`
                (:`OnConfirm`
                  (bind _returnvalue (`AuraAbilitySystemLibrary.GetHighLightedActor` null))
                  (bind _output_get (set `self.HighlightedActor` _returnvalue))
                  (`/Engine/EditorBlueprintResources/StandardMacros.IsValid` _output_get
                    (:`Is Valid`
                      (if (`KismetSystemLibrary.DoesImplementInterface` _highlightedactor "/Script/Aura.AllyInterface")
                        (message `CombatInterface.UpdateFacingTarget` (`self.GetAvatarActorFromActorInfo`) (`Actor.K2_GetActorLocation` _highlightedactor))
                        (`AbilityTask_PlayMontageAndWait.CreatePlayMontageAndWaitProxy` "None" "/Game/Assets/Characters/Aura/Animations/Abilities/AM_Cast_EnchantConfirm.AM_Cast_EnchantConfirm" 1.0 "None" false
                          (:`then`
                            (`AbilityTask_WaitGameplayEvent.WaitGameplayEvent` (struct :`TagName` "Event.Montage.ConfirmEnchant") null
                              (:`EventReceived`
                                (`self.EnchantAlly` (`self.HighlightedActor`))
                                (`self.K2_CommitAbility`)))))))
                    (:`Is Not Valid`
                      _)))
                (:`OnCancel`
                  _))
              (`self.PrepareToEnd`)
              (`self.K2_EndAbility`))))))))

(event `self.K2_OnEndAbility`
  (params (bWasCancelled :type Boolean)))

(fn `InCastingLoop`
  (bind _charactermovement (`Character.CharacterMovement` (`self.OwnerCharacter`)))
  (message `CombatInterface.SetIsCastingLoop` (`self.GetAvatarActorFromActorInfo`) true)
  (set `self.OriginalMaxWalkSpeed` (`CharacterMovementComponent.MaxWalkSpeed` _charactermovement))
  (set `CharacterMovementComponent.MaxWalkSpeed` 0.0 _charactermovement))

(fn `PrepareToEnd`
  (message `CombatInterface.SetIsCastingLoop` (`self.GetAvatarActorFromActorInfo`) false)
  (`CharacterMovementComponent.SetMovementMode` (`Character.CharacterMovement` (`self.OwnerCharacter`)) "MOVE_Walking" 0)
  (set `CharacterMovementComponent.MaxWalkSpeed` (`self.OriginalMaxWalkSpeed`) (`Character.CharacterMovement` (`self.OwnerCharacter`)))
  (`self.ChangeToLiriaInputMapping`))