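; GA_ArcaneEnchant is a gameplay ability for Aura's Arcane enchant, currently a debug-print skeleton with no enchant effect.
; On activation it waits for input release, then switches to a confirm input mapping context and waits for confirm or cancel.
; Confirm commits the ability, while cancel skips the commit.
; Both paths restore the Liria mapping context and end the ability.
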(event `self.K2_ActivateAbility`
  (`AbilityTask_WaitInputRelease.WaitInputRelease` false
    (:`OnRelease`
      (`AuraAbilitySystemLibrary.ChangeToConfirmImc` self)
      (`AbilityTask_WaitConfirmCancel.WaitConfirmCancel`
        (:`OnConfirm`
          (`KismetSystemLibrary.PrintString` "ARCANE EXECUTED")
          (`self.K2_CommitAbility`))
        (:`OnCancel`
          (`KismetSystemLibrary.PrintString` "ARCANE CANCELLED" true true (struct :`R` 1.0 :`B` 0.100554 :`A` 1.0))))
      (`AuraAbilitySystemLibrary.ChangeToLiriaImc` self)
      (`self.K2_EndAbility`))))

(event `self.K2_OnEndAbility`
  (params (bWasCancelled :type Boolean))
  (`KismetSystemLibrary.PrintString` "end ability enchant"))