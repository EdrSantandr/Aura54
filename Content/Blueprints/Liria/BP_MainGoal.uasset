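; BP_MainGoal is the main goal actor, apparently a tree, with an event that plays its dark destruction effect.
; SetDarkLightning plays a cracking sound, turns the spotlight a dim reddish color and activates the explosion effect.
; A timeline then reduces the mesh's uniform scale from its starting Z scale by a ScaleTree-weighted amount, hiding the mesh when finished.
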(event `self.SetDarkLightning`
  (bind (_initialscale_x _initialscale_y _initialscale_z) (`KismetMathLibrary.BreakVector` (`self.InitialScale`)))
  (`GameplayStatics.SpawnSound2D` (`self.CrackingSound`) 1.0 1.0 0.0 null)
  (`LightComponent.SetLightColor` (`self.SpotLight`) (make `LinearColor` 0.020833 0.0 0.010939) true)
  (set `self.InitialScale` (`SceneComponent.K2_GetComponentScale` (`self.MainGoalMesh`)))
  (`ActorComponent.Activate` (`self.N_TreeExplosion`) true)
  (bind (_direction _scale) (`Timeline|MeshTreeTimeline` :!via `PlayFromStart`)
    (:`Update`
      (`SceneComponent.SetRelativeScale3D` (`self.MainGoalMesh`) (`KismetMathLibrary.Conv_DoubleToVector` (- _initialscale_z (* _scale (`self.ScaleTree`))))))
    (:`Finished`
      (`SceneComponent.SetHiddenInGame` (`self.MainGoalMesh`) true false))))

(fn `UserConstructionScript`)