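; GA_Sentinel_Blackbolt is an arcane gameplay ability that lets an allied Sentinel fire homing projectiles at its combat target.
; On activation it turns the avatar toward the target and sends the target location to a mesh scale-and-rotate message.
; It then spawns spread projectiles from a point offset from the avatar based on the target's position, with a fixed pitch override and homing on the target.
; The ability ends immediately after spawning.
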(event `self.K2_ActivateAbility`
  (bind _returnvalue (`Actor.K2_GetActorLocation` (`self.CombatTarget`)))
  (bind _output_get (set `self.AvatarActor` (`self.GetAvatarActorFromActorInfo`)))
  (bind _returnvalue_2 (message `EnemyInterface.GetCombatTarget` _output_get))
  (set `self.CombatTarget` _returnvalue_2)
  (message `CombatInterface.UpdateFacingTarget` (`self.AvatarActor`) _returnvalue)
  (bind _output_get_2 (set `self.ProjectileTargetLocation` _returnvalue))
  (message `CombatInterface.ScalingRotatingMesh` (`self.AvatarActor`) _output_get_2)
  (bind _returnvalue_3 (`self.GetSpawnProjectileLocationPoint` (`Actor.K2_GetActorLocation` (`self.AvatarActor`)) (`self.ProjectileTargetLocation`)))
  (`self.SpawnSpreadProjectilesWithOrigin` (`self.ProjectileTargetLocation`) _returnvalue_3 true 15.0 (`self.CombatTarget`))
  (`self.K2_EndAbility`))