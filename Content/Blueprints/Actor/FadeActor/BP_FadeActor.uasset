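; BP_FadeActor is a static mesh actor that fades out and back in through a material parameter.
; Construction caches original materials and builds dynamic instances from FadeMaterials.
; FadeOut applies those instances and plays a timeline driving their Fade scalar, while Fadein reverses it.
; On finish, full Fade restores original materials, and BlockVisibility optionally toggles Visibility-channel collision between Block at full and Ignore at zero.
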(event `/Game/Blueprints/Actor/FadeActor/BI_FadeInterface.FadeOut`
  (`self.SetMaterialsToDynamicInstances`)
  (bind (_direction _fadeamount) (`Timeline|FadeTimeline` :!label _label)
    (:`Update`
      (for _array_element (`self.DynamicMaterials`)
        (`MaterialInstanceDynamic.SetScalarParameterValue` _array_element "Fade" _fadeamount)))
    (:`Finished`
      (`self.FadeFinished` _fadeamount))))

(event `/Game/Blueprints/Actor/FadeActor/BI_FadeInterface.FadeIn`
  (goto _label :!via `Reverse`))

(event `self.ReceiveBeginPlay`)

(fn `FadeFinished`
  (params (A :type "Float (double-precision)"))
  (if (>= A 1.0)
    (`self.ResetMaterials`)
    (if (`self.BlockVisibility`)
      (`PrimitiveComponent.SetCollisionResponseToChannel` (`self.StaticMesh`) "ECC_Visibility" "ECR_Block"))
    (elif (<= A 0.0)
      (if (`self.BlockVisibility`)
        (`PrimitiveComponent.SetCollisionResponseToChannel` (`self.StaticMesh`) "ECC_Visibility" "ECR_Ignore")))))

(fn `ResetMaterials`
  (for (_array_element _array_index) (`self.OriginalMaterials`)
    (`PrimitiveComponent.SetMaterial` (`self.StaticMesh`) _array_index _array_element)))

(fn `SetMaterialsToDynamicInstances`
  (for (_array_element _array_index) (`self.DynamicMaterials`)
    (`PrimitiveComponent.SetMaterial` (`self.StaticMesh`) _array_index _array_element)))

(fn `UserConstructionScript`
  (`KismetArrayLibrary.Array_Clear` (`self.DynamicMaterials`))
  (set `self.OriginalMaterials` (`MeshComponent.GetMaterials` (`self.StaticMesh`)))
  (for _array_element (`self.FadeMaterials`)
    (bind _returnvalue (`KismetMaterialLibrary.CreateDynamicMaterialInstance` _array_element))
    (`KismetArrayLibrary.Array_AddUnique` (`self.DynamicMaterials`) _returnvalue)))