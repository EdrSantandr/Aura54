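; Strong variant of the Sentinel base ally actor, which adds a procedural animation to its mesh.
; BeginPlay disables mesh collision, caches the original scale and picks a random rotation magnitude.
; A timeline then drives vertical movement, scale relative to the original and incremental yaw rotation.
; World Z is set directly from the curve times ZTraslation, not offset from the starting height.
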(event `self.ReceiveBeginPlay`
  (bind _meshcomponent (`self.MeshComponent`))
  (bind _meshcomponent_2 (`self.MeshComponent`))
  (bind (_returnvalue_x _returnvalue_y) (`KismetMathLibrary.BreakVector` (`SceneComponent.K2_GetComponentLocation` _meshcomponent)))
  (`parent.ReceiveBeginPlay`)
  (`PrimitiveComponent.SetCollisionEnabled` _meshcomponent_2 "NoCollision")
  (set `self.OriginalScale` (`SceneComponent.K2_GetComponentScale` _meshcomponent_2))
  (set `self.RotationMagnitude` (`KismetMathLibrary.RandomFloatInRange` (`self.MinRotation`) (`self.MaxRotation`)))
  (bind (_direction _scale _rotation _zmovement) (`Timeline|RotAndScaleTimeline` :!via `PlayFromStart`)
    (:`Update`
      (`|ExecutionSequence`
        (:`then_0`
          (`SceneComponent.K2_SetWorldLocation` _meshcomponent (`KismetMathLibrary.MakeVector` _returnvalue_x _returnvalue_y (* _zmovement (`self.ZTraslation`))) false false))
        (:`then_1`
          (`SceneComponent.SetWorldScale3D` (`self.MeshComponent`) (* (`self.OriginalScale`) _scale)))
        (:`then_2`
          (`SceneComponent.K2_AddWorldRotation` (`self.MeshComponent`) (`KismetMathLibrary.MakeRotator` 0.0 0.0 (* _rotation (`self.RotationMagnitude`))) false false))))))

(fn `UserConstructionScript`
  (`parent.UserConstructionScript`))