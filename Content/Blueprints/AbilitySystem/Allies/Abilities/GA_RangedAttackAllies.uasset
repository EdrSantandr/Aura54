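; Gameplay ability for allies that fires a ranged projectile at the avatar's combat target.
; On activation it turns the avatar toward the target and triggers a scaling/rotating mesh through messages, then waits briefly.
; If the re-fetched target is still valid, it spawns a homing projectile slightly ahead of the avatar along the target direction, with optional pitch override.
; The ability then ends.
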(event `self.K2_ActivateAbility`
  (bind _returnvalue (`self.GetAvatarActorFromActorInfo`))
  (bind _returnvalue_2 (`self.GetAvatarActorFromActorInfo`))
  (bind _returnvalue_3 (message `EnemyInterface.GetCombatTarget` _returnvalue_2))
  (bind _returnvalue_4 (`Actor.K2_GetActorLocation` _returnvalue_3))
  (message `CombatInterface.UpdateFacingTarget` _returnvalue_2 _returnvalue_4)
  (message `CombatInterface.ScalingRotatingMesh` _returnvalue_2 _returnvalue_4)
  (`KismetSystemLibrary.Delay` 0.5)
  (bind _returnvalue_5 (message `EnemyInterface.GetCombatTarget` _returnvalue))
  (`/Engine/EditorBlueprintResources/StandardMacros.IsValid` _returnvalue_5
    (:`Is Valid`
      (`self.SpawnProjectileAtLocation` _returnvalue_5 (`self.GetSpawnLocationPoint` (`Actor.K2_GetActorLocation` _returnvalue) (`Actor.K2_GetActorLocation` _returnvalue_5) 50.0) (`self.ShouldOverridePitch`) (`self.PitchOverride`)))
    (:`Is Not Valid`
      _))
  (`self.K2_EndAbility`))

(fn `GetSpawnLocationPoint`
  (params (ActorLocation :type "Vector Structure") (EnemyLocation :type "Vector Structure") (Distance :type "Float (double-precision)"))
  (returns (SpawnLocation :type "Vector Structure"))
  (return (+ ActorLocation (* (`KismetMathLibrary.Normal` (- EnemyLocation ActorLocation)) Distance))))