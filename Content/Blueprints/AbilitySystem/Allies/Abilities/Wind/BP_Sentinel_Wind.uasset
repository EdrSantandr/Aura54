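; Wind projectile for the Sentinel ally ability that has a random chance to disarm what it hits.
; On hit, targets implementing CombatInterface can receive a timed disarm message.
; Its sphere collision switches to query-only shortly after BeginPlay.
; Each tick it compares its position with the last frame and, when it has nearly stopped, plays fire impact sound and explosion effects, then destroys itself.
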(event `self.ReceiveBeginPlay`
  (`KismetSystemLibrary.Delay` 0.1)
  (bind _spherecomponent (`self.SphereComponent`)
    (:`then`
      (`PrimitiveComponent.SetCollisionEnabled` _spherecomponent "QueryOnly"))
    (:`else`)))

(event `self.ReceiveTick`
  (params (DeltaSeconds :type "Float (single-precision)"))
  (`self.AutomaticallyDestroyed`))

(event `self.OnHitProjectile`
  (params (InOtherActor :type "Actor Object Reference"))
  (bind _output_get (set `self.HitActor` (`|ConvertAsset` InOtherActor)))
  (if (`KismetSystemLibrary.DoesImplementInterface` (`|ConvertAsset` _output_get) "/Script/Aura.CombatInterface")
    (if (<= (`KismetMathLibrary.RandomFloatInRange` 0.0 1.0) (`self.DisarmEffectChance`))
      (message `CombatInterface.StartDisarm` (`|ConvertAsset` (`self.HitActor`)) (`self.DisarmEffectDuration`)))))

(fn `AutomaticallyDestroyed`
  (set `self.LocationLastFrame` (`self.LocationThisFrame`))
  (set `self.LocationThisFrame` (`self.K2_GetActorLocation`))
  (if (<= (`KismetMathLibrary.VSize` (- (`self.LocationThisFrame`) (`self.LocationLastFrame`))) (`self.MinDistancePerFrame`))
    (`GameplayStatics.SpawnSoundAtLocation` "/Game/Assets/Sounds/Abilities/FireBolt/sfx_FireBolt_Impact.sfx_FireBolt_Impact" (`self.LocationThisFrame`) (struct) 1.0 1.0 0.0 null null)
    (`NiagaraFunctionLibrary.SpawnSystemAtLocation` "/Game/Assets/Effects/Projectiles/FireExplosion/NS_FireExplosion1.NS_FireExplosion1" (`self.LocationThisFrame`))
    (`self.K2_DestroyActor`)))

(fn `UserConstructionScript`)