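; Invoke gameplay ability that summons a Sentinel actor with its default controller in front of the caster.
; On input release it checks cost, zeroes walk speed and plays the cast montage.
; The montage's gameplay event triggers the spawn, restores speed, then commits and ends the ability.
; Helper functions gather enemies in a radius and apply radial knockback damage, but the event graph never calls them.
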(event `self.K2_ActivateAbility`
  (bind _ownercharacter (`self.OwnerCharacter`))
  (`KismetSystemLibrary.PrintString` "invoke")
  (`AbilityTask_WaitInputRelease.WaitInputRelease` false
    (:`OnRelease`
      (bind _returnvalue (`self.K2_CheckAbilityCost`))
      (if _returnvalue
        (bind _ascharacter (cast `Character` (`self.GetAvatarActorFromActorInfo`)))
        (bind _output_get (set `self.OwnerCharacter` _ascharacter))
        (bind _charactermovement (`Character.CharacterMovement` _output_get))
        (set `self.OriginalMaxWalkSpeed` (`MovementComponent.GetMaxSpeed` _charactermovement))
        (set `CharacterMovementComponent.MaxWalkSpeed` 0.0 _charactermovement)
        (`AbilityTask_PlayMontageAndWait.CreatePlayMontageAndWaitProxy` "None" "/Game/Assets/Characters/Aura/Animations/Abilities/AM_Cast_Invoke.AM_Cast_Invoke"
          (:`then`
            (`AbilityTask_WaitGameplayEvent.WaitGameplayEvent` (struct :`TagName` "Event.Montage.Invoke") null true
              (:`EventReceived`
                (bind _returnvalue_2 (`|SpawnActorFromClass` (`self.SentinelClass`) (`KismetMathLibrary.MakeTransform` (+ (`Actor.K2_GetActorLocation` _ownercharacter) (* (`Actor.GetActorForwardVector` _ownercharacter) (`self.Distance`)))) "AdjustIfPossibleButAlwaysSpawn" "MultiplyWithRoot" _ownercharacter null))
                (bind _output_get_2 (set `self.SentinelSpawned` _returnvalue_2))
                (`Pawn.SpawnDefaultController` _output_get_2)
                (set `CharacterMovementComponent.MaxWalkSpeed` (`self.OriginalMaxWalkSpeed`) (`Character.CharacterMovement` (`self.OwnerCharacter`)))
                (`self.K2_CommitAbility`)
                (`self.K2_EndAbility`)))))))))

(fn `RadialDamageToPlayer`
  (params (TargetActor :type "Actor Object Reference"))
  (bind _returnvalue (- (`Actor.K2_GetActorLocation` TargetActor) (`self.SphereSpawnLocation`)))
  (`AuraAbilitySystemLibrary.ApplyDamageEffect` (`self.MakeDamageEffectParamsFromClassDefaults` TargetActor (`self.SphereSpawnLocation`) true _returnvalue true _returnvalue true 25.0)))

(fn `StorePlayersToDamage`
  (bind _returnvalue (`self.GetAvatarActorFromActorInfo`))
  (bind _outoverlappedactors (`AuraAbilitySystemLibrary.GetLiveEnemiesWithinRadius` _returnvalue (`|MakeArray` _returnvalue) (`self.RadialDamageOuterRadius`) (`self.SphereSpawnLocation`)))
  (set `self.PlayersToDamage` _outoverlappedactors))