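; Wind wave ability actor that disarms enemies it overlaps and drags them horizontally while it lives.
; A size timeline grows it, then an explosion effect and implosion timeline scale it down before it clears disarms and destroys itself.
; Tick shifts caught enemies along the direction from LocationLastFrame, which stays at world origin because HandleAttraction self-assigns it.
; AutomaticallyDestroyed, a stall check with fire effects, is never called here.
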(event `self.ReceiveBeginPlay`
  (set `self.LocationThisFrame` (0.0 0.0 0.0))
  (set `self.LocationLastFrame` (0.0 0.0 0.0))
  (bind _spherecomponent (`self.SphereComponent`)
    (:`then`
      (`PrimitiveComponent.SetCollisionEnabled` _spherecomponent "QueryOnly")
      (`TimelineComponent.SetPlayRate` (`self.SizeTimeline`) (`KismetMathLibrary.SafeDivide` 1.0 (`self.SizeTimelineDuration`)))
      (bind (_direction _size) (`Timeline|SizeTimeline`)
        (:`Update`
          (`self.SetActorScale3D` (`KismetMathLibrary.Conv_DoubleToVector` _size)))
        (:`Finished`
          (`NiagaraFunctionLibrary.SpawnSystemAtLocation` (`self.NiagarraExplotion`) (`self.K2_GetActorLocation`))
          (set `self.OriginalScale` (`self.GetActorScale3D`))
          (bind (_direction_2 _scale) (`Timeline|ImplosionTimeline` :!via `PlayFromStart`)
            (:`Update`
              (`self.SetActorScale3D` (* (`self.OriginalScale`) _scale)))
            (:`Finished`
              (for _array_element (`self.ActorsDisarmed`)
                (bind _output (`|ConvertAsset` _array_element))
                (if (`KismetSystemLibrary.DoesImplementInterface` _output "/Script/Aura.CombatInterface")
                  (message `CombatInterface.SetIsDisarmed` _output false)))
              (`KismetArrayLibrary.Array_Clear` (`self.ActorsDisarmed`))
              (`self.K2_DestroyActor`))))))
    (:`else`)))

(event `self.ReceiveTick`
  (params (DeltaSeconds :type "Float (single-precision)"))
  (if (> (`KismetArrayLibrary.Array_Length` (`self.ActorsDisarmed`)) 0)
    (`self.HandleAttraction` DeltaSeconds)))

(event `self.SphereComponent.OnComponentBeginOverlap`
  (params (OverlappedComponent :type "PrimitiveComponent Object Reference") (OtherActor :type "Actor Object Reference") (OtherComp :type "PrimitiveComponent Object Reference") (OtherBodyIndex :type Integer) (bFromSweep :type Boolean) (SweepResult :type "HitResult Structure (by ref)"))
  (bind _hitactor (`self.HitActor`))
  (bind _output_get (set `self.HitActor` (`|ConvertAsset` OtherActor)))
  (if (`KismetSystemLibrary.DoesImplementInterface` (`|ConvertAsset` _output_get) "/Script/Aura.EnemyInterface")
    (`KismetArrayLibrary.Array_AddUnique` (`self.ActorsDisarmed`) _hitactor)
    (message `CombatInterface.StartDisarm` (`|ConvertAsset` _hitactor) (`self.SizeTimelineDuration`) false)))

(fn `AutomaticallyDestroyed`
  (set `self.LocationLastFrame` (`self.LocationThisFrame`))
  (set `self.LocationThisFrame` (`self.K2_GetActorLocation`))
  (if (<= (`KismetMathLibrary.VSize` (- (`self.LocationThisFrame`) (`self.LocationLastFrame`))) (`self.MinDistancePerFrame`))
    (`GameplayStatics.SpawnSoundAtLocation` "/Game/Assets/Sounds/Abilities/FireBolt/sfx_FireBolt_Impact.sfx_FireBolt_Impact" (`self.LocationThisFrame`) (struct) 1.0 1.0 0.0 null null)
    (`NiagaraFunctionLibrary.SpawnSystemAtLocation` "/Game/Assets/Effects/Projectiles/FireExplosion/NS_FireExplosion1.NS_FireExplosion1" (`self.LocationThisFrame`))
    (`self.K2_DestroyActor`)))

(fn `HandleAttraction`
  (params (Delta :type "Float (double-precision)"))
  (locals (PositionZ :type "Float (double-precision)") (PositionY :type "Float (double-precision)") (PositionX :type "Float (double-precision)") (DirectionInteraction :type "Vector Structure") (IntervalMagnitude :type "Float (double-precision)"))
  (bind (_returnvalue_x _returnvalue_y) (`KismetMathLibrary.BreakVector` (* (`local.DirectionInteraction`) (* (`self.AttractionForce`) Delta))))
  (set `self.LocationLastFrame` (`self.LocationLastFrame`))
  (set `self.LocationThisFrame` (`self.K2_GetActorLocation`))
  (set `local.DirectionInteraction` (`KismetMathLibrary.Normal` (- (`self.LocationThisFrame`) (`self.LocationLastFrame`))))
  (for _array_element (`self.ActorsDisarmed`)
    (bind _output (`|ConvertAsset` _array_element))
    (bind (_returnvalue_x_2 _returnvalue_y_2 _returnvalue_z) (`KismetMathLibrary.BreakVector` (`self.K2_GetActorLocation` _output)))
    (`self.K2_SetActorLocation` _output (`KismetMathLibrary.MakeVector` (+ _returnvalue_x_2 _returnvalue_x) (+ _returnvalue_y_2 _returnvalue_y) _returnvalue_z) false false)))

(fn `UserConstructionScript`)