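; Base enemy character Blueprint handling spawn scale-in, death loot drops, dissolve visuals and attack facing.
; SpawnLoot pulls items from the loot tiers info, then a looping timer spawns them one at a time at shuffled, evenly spread rotations and random distances, optionally matching enemy level.
; Timelines drive optional spawn scaling and mesh and weapon dissolve material parameters.
; UpdateFacingTarget feeds the FacingTarget motion warp target.
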(event `self.SpawnLoot`
  (bind _returnvalue (`AuraAbilitySystemLibrary.GetLootTiersInfo` null))
  (`/Engine/EditorBlueprintResources/StandardMacros.IsValid` _returnvalue
    (:`Is Valid`
      (bind _returnvalue_2 (`LootTiersInfo.GetLootItems` _returnvalue))
      (bind _output_get (set `self.LootItems` _returnvalue_2))
      (set `self.LootRotations` (`self.GetLootRotations` _output_get))
      (`KismetArrayLibrary.Array_Shuffle` (`self.LootRotations`))
      (set `self.SpawnLootCount` 0)
      (bind _returnvalue_3 (`KismetSystemLibrary.K2_SetTimerDelegate` (delegate `SpawnLootItem`) 0.1 true))
      (set `self.LootTimer` _returnvalue_3)
      (`self.SpawnLootItem`))))

(event `SpawnLootItem`
  (bind (_lootclass _blootleveloverride) (break `LootItem` (`|GetArrayItem` (`self.LootItems`) (`self.SpawnLootCount`))))
  (if (< (`self.SpawnLootCount`) (`KismetArrayLibrary.Array_Length` (`self.LootItems`)))
    (set `self.SpawnDistance` (`KismetMathLibrary.RandomFloatInRange` (`self.MinSpawnDistance`) (`self.MaxSpawnDistance`)))
    (bind _returnvalue (`|SpawnActorFromClass` _lootclass (`self.GetLootTransform` (`self.SpawnLootCount`) (`self.SpawnDistance`)) "AlwaysSpawn" "MultiplyWithRoot" null null))
    (bind _asaura_effect_actor (cast `AuraEffectActor` _returnvalue))
    (if (and (`KismetSystemLibrary.IsValid` _asaura_effect_actor) _blootleveloverride)
      (set `AuraEffectActor.ActorLevel` (`KismetMathLibrary.Conv_IntToDouble` (`self.Level`)) _asaura_effect_actor))
    (`/Engine/EditorBlueprintResources/StandardMacros.IncrementInt` (`self.SpawnLootCount`))
    (else
      (`KismetSystemLibrary.K2_ClearAndInvalidateTimerHandle` (`self.LootTimer`)))))

(event `self.ReceiveBeginPlay`
  (if (`self.SpawnScaleEffect`)
    (bind (_direction _scaletrack) (`Timeline|SpawnTimeline`)
      (:`Update`
        (`SceneComponent.SetRelativeScale3D` (`self.Mesh`) (`KismetMathLibrary.MakeVector` _scaletrack _scaletrack _scaletrack))))))

(event `self.StartMeshDissolveTimeline`
  (params (DynamicMaterialInstance :type "MaterialInstanceDynamic Object Reference"))
  (bind (_direction _dissolvetrack) (`Timeline|DissolveMeshTimeline`)
    (:`Update`
      (`MaterialInstanceDynamic.SetScalarParameterValue` DynamicMaterialInstance "Dissolve" _dissolvetrack))))

(event `self.StartWeaponDissolveTimeline`
  (params (DynamicMaterialInstance :type "MaterialInstanceDynamic Object Reference"))
  (bind (_direction _dissolveweapon) (`Timeline|DissolveWeaponTimeline`)
    (:`Update`
      (`MaterialInstanceDynamic.SetScalarParameterValue` DynamicMaterialInstance "Dissolve" _dissolveweapon))))

(event `CombatInterface.UpdateFacingTarget`
  (params (Target :type "Vector Structure (by ref)"))
  (`MotionWarpingComponent.AddOrUpdateWarpTargetFromLocation` (`self.MotionWarping`) "FacingTarget" Target))

(fn `GetLootRotations`
  (params (TargetArray :type "Array of LootItem Structure (by ref)"))
  (returns (ReturnValue :type "Array of Rotator Structure"))
  (return (`AuraAbilitySystemLibrary.EvenlySpreadRotators` (`self.GetActorForwardVector`) (`KismetMathLibrary.Vector_Up`) 360.0 (`KismetArrayLibrary.Array_Length` TargetArray))))

(fn `GetLootTransform`
  (params (LootCount :type Integer) (SpawnDistance :type "Float (single-precision)"))
  (returns (SpawnTransform :type "Transform Structure"))
  (bind _output (`|GetArrayItem` (`self.LootRotations`) LootCount))
  (return (`KismetMathLibrary.MakeTransform` (+ (* (`KismetMathLibrary.GetForwardVector` _output) SpawnDistance) (`self.K2_GetActorLocation`)) _output)))

(fn `UserConstructionScript`)