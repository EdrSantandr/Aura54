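; Base Blueprint for ally characters, providing a mesh turn-and-scale effect toward a given target.
; ScalingRotatingMesh snaps the mesh to a look-at rotation computed from the actor's forward vector, rather than its location, to the target.
; It stores the mesh's relative scale, adds a timeline curve scaled by ScalePercentage while playing, then restores the stored scale when finished.
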(event `CombatInterface.ScalingRotatingMesh`
  (params (Target :type "Vector Structure (by ref)"))
  (`SceneComponent.K2_SetWorldRotation` (`self.MeshComponent`) (`KismetMathLibrary.FindLookAtRotation` (`self.GetActorForwardVector`) Target) false false)
  (set `self.RelativeScale` (`SceneComponent.RelativeScale3D` (`self.MeshComponent`)))
  (bind (_direction _scale) (`Timeline|ScaleTimeline` :!via `PlayFromStart`)
    (:`Update`
      (`SceneComponent.SetRelativeScale3D` (`self.MeshComponent`) (+ (`self.RelativeScale`) (* _scale (`self.ScalePercentage`)))))
    (:`Finished`
      (`SceneComponent.SetRelativeScale3D` (`self.MeshComponent`) (`self.RelativeScale`)))))

(fn `UserConstructionScript`)