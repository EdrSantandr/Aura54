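; GA_Meteor is a meteor gameplay ability that currently only prints a debug message on activation.
; An unconnected chain waits for input release, plays a cast montage, roots the caster in a casting loop and switches to confirm/cancel input.
; On confirm with a highlighted enemy, it turns the caster, fires homing spread projectiles on a montage event and commits.
; PrepareToEnd restores movement and input before the ability ends.
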(event `self.K2_ActivateAbility`
  (`KismetSystemLibrary.PrintString` "meteor activated"))

(fn `InCastingLoop`
  (bind _charactermovement (`Character.CharacterMovement` (`self.OwnerCharacter`)))
  (message `CombatInterface.SetIsCastingLoop` (`self.GetAvatarActorFromActorInfo`) true)
  (set `self.OriginalMaxWalkSpeed` (`CharacterMovementComponent.MaxWalkSpeed` _charactermovement))
  (set `CharacterMovementComponent.MaxWalkSpeed` 0.0 _charactermovement))

(fn `PrepareToEnd`
  (bind _charactermovement (`Character.CharacterMovement` (`self.OwnerCharacter`)))
  (message `CombatInterface.SetIsCastingLoop` (`self.GetAvatarActorFromActorInfo`) false)
  (`CharacterMovementComponent.SetMovementMode` _charactermovement "MOVE_Walking" 0)
  (set `CharacterMovementComponent.MaxWalkSpeed` (`self.OriginalMaxWalkSpeed`) _charactermovement)
  (`self.ChangeToLiriaInputMapping`))