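; Gameplay ability for the Arcane Black Hole Bolt, which fires spread projectiles from the avatar's weapon socket.
; On activation it targets a point a set distance along the avatar's forward vector and plays the cast montage.
; A montage gameplay event triggers the inherited spread-projectile spawn, then commits and ends the ability.
; Montage completion, blend-out, interruption or cancellation also ends it.
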(event `self.K2_ActivateAbility`
  (set `self.AvatarActor` (`self.GetAvatarActorFromActorInfo`))
  (bind _finallocation (`self.CreateProjectileLocation`))
  (set `self.ProjectileTargetLocation` _finallocation)
  (`AbilityTask_PlayMontageAndWait.CreatePlayMontageAndWaitProxy` "None" "/Game/Assets/Characters/Aura/Animations/Abilities/AM_Cast_BlackHoleBolt.AM_Cast_BlackHoleBolt"
    (:`then`
      (`AbilityTask_WaitGameplayEvent.WaitGameplayEvent` (struct :`TagName` "Event.Montage.BlackHoleBolt") null
        (:`EventReceived`
          (`self.SpawnSpreadProjectiles` (`self.ProjectileTargetLocation`) (`BlueprintGameplayTagLibrary.MakeLiteralGameplayTag` (struct :`TagName` "CombatSocket.Weapon")))
          (`self.K2_CommitAbility`)
          (`self.K2_EndAbility`))))
    (:`OnCompleted`
      (`self.K2_EndAbility` :!label _label))
    (:`OnBlendOut`
      (goto _label))
    (:`OnInterrupted`
      (goto _label))
    (:`OnCancelled`
      (goto _label))))

(fn `CreateProjectileLocation`
  (returns (FinalLocation :type "Vector Structure"))
  (bind _avataractor (`self.AvatarActor`))
  (return (+ (`Actor.K2_GetActorLocation` _avataractor) (* (`Actor.GetActorForwardVector` _avataractor) (`self.Distance`)))))